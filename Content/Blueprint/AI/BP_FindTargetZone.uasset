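; Behavior Tree task that picks a random target zone for an AI.
; It fetches all BP_Zone actors, picks one at random and writes it to the blackboard key before finishing successfully.
; Invalid picks, including the out-of-range index the random range allows, and enemy spawner zones loop back to a fresh search.
; The retry has no limit or failure path.
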(event EventReceiveExecuteAI
  (params (OwnerController :type AI%20Controller%20Object%20Reference) (ControlledPawn :type Pawn%20Object%20Reference))
  (bind _outactors (Actor|GetAllActorsOfClass "/Game/Blueprint/BP_Zone.BP_Zone_C" :!label _label))
  (bind _output_get (Variables|Default|SetLocal (Utilities|Array|Get(acopy) _outactors (Math|Random|RandomIntegerinRange 0 (Utilities|Array|Length _outactors)))))
  (Utilities|IsValid _output_get
    (:Is%20Valid
      (if (== (Variables|/Game/Blueprint/BP_Zone.BP_Zone_C|GetIsEnemySpawner _output_get) false)
        (Class|BTFunctionLibrary|SetBlackboardValueasObject (Variables|Default|GetKey) (Variables|Default|GetLocal))
        (AI|BehaviorTree|FinishExecute true)
        (else
          (goto _label))))
    (:Is%20Not%20Valid
      (goto _label))))