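; BP_Zone is a team zone that acts as either an enemy spawner or an enemy removal area, chosen by IsEnemySpawner.
; As a spawner, it uses a Delay on Tick to spawn a BP_EnemyTeam every two seconds near its location.
; Otherwise, its box overlap destroys any BP_EnemyTeam that enters.
; The construction script tints the decal's dynamic material and spawn FX with the enemy or player color.
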(event OnComponentBeginOverlap(Box)
  (params (OverlappedComponent :type Primitive%20Component%20Object%20Reference) (OtherActor :type Actor%20Object%20Reference) (OtherComp :type Primitive%20Component%20Object%20Reference) (OtherBodyIndex :type Integer) (bFromSweep :type Boolean) (SweepResult :type Hit%20Result%20Structure%20%28by%20ref%29))
  (if (not (Variables|Default|GetIsEnemySpawner))
    (bind _asbp_enemy_team (Utilities|Casting|CastToBP_EnemyTeam OtherActor))
    (Actor|DestroyActor _asbp_enemy_team)))

(event EventBeginPlay)

(event Collision|EventActorBeginOverlap
  (params (OtherActor :type Actor%20Object%20Reference)))

(event EventTick
  (params (DeltaSeconds :type Float%20%28single-precision%29))
  (if (Variables|Default|GetIsEnemySpawner)
    (Utilities|FlowControl|Delay 2.0)
    (Game|SpawnActorfromClass "/Game/Blueprint/BP_EnemyTeam.BP_EnemyTeam_C" (Math|Conversions|ToTransform(Vector) (+ (Transformation|GetActorLocation) 1e+02)) "AlwaysSpawn" "MultiplyWithRoot" 0 0)))

(fn ConstructionScript
  (bind _isenemyspawner (Variables|Default|GetIsEnemySpawner))
  (bind _enemycolor (Variables|Default|GetEnemyColor))
  (bind _playercolor (Variables|Default|GetPlayerColor))
  (bind _returnvalue (Math|Color|SelectColor _enemycolor _playercolor _isenemyspawner))
  (Utilities|IsValid (Variables|Default|GetDynMat)
    (:Is%20Valid
      _)
    (:Is%20Not%20Valid
      (bind _returnvalue_2 (Rendering|Material|CreateDynamicMaterialInstance "/Game/Materials/M_Zone_Inst.M_Zone_Inst" "None" "None" :!class /Script/Engine.KismetMaterialLibrary))
      (Variables|Default|SetDynMat _returnvalue_2)))
  (Effects|Components|ParticleSystem|SetColorParameter (Variables|Default|GetFX_Spawn) "Color" _returnvalue)
  (Rendering|Material|SetVectorParameterValue (Variables|Default|GetDynMat) "Color" _returnvalue :!class /Script/Engine.MaterialInstanceDynamic)
  (Rendering|Components|Decal|SetDecalMaterial (Variables|Default|GetDecal) (Variables|Default|GetDynMat)))