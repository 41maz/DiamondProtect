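; BP_PlayerTeam is a player-side unit that automatically faces and shoots at enemies.
; A sphere overlap stores the latest BP_EnemyTeam actor as Target, with no end-overlap clearing.
; While Target is valid, Tick yaws the actor toward it with a small offset.
; A Delay in Tick paces firing to roughly twice a second, spawning BP_Projectile at the Scene component with velocity aimed at Target.
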(event OnComponentBeginOverlap(Sphere)
  (params (OverlappedComponent :type Primitive%20Component%20Object%20Reference) (OtherActor :type Actor%20Object%20Reference) (OtherComp :type Primitive%20Component%20Object%20Reference) (OtherBodyIndex :type Integer) (bFromSweep :type Boolean) (SweepResult :type Hit%20Result%20Structure%20%28by%20ref%29))
  (bind _asbp_enemy_team (Utilities|Casting|CastToBP_EnemyTeam OtherActor))
  (Variables|Default|SetTarget _asbp_enemy_team))

(event EventBeginPlay)

(event EventTick
  (params (DeltaSeconds :type Float%20%28single-precision%29))
  (bind _target (Variables|Default|GetTarget))
  (Utilities|IsValid _target
    (:Is%20Valid
      (Transformation|SetActorRotation (Math|Rotator|MakeRotator 0.0 0.0 (+ (.yaw (Math|Rotator|FindLookatRotation (Transformation|GetActorLocation) (Transformation|GetActorLocation _target))) -5.0)))
      (Utilities|FlowControl|Delay 0.5)
      (bind _returnvalue (Game|SpawnActorfromClass "/Game/Blueprint/BP_Projectile.BP_Projectile_C" (Transformation|GetWorldTransform (Variables|Default|GetScene)) "Undefined" "MultiplyWithRoot" 0 0))
      (Variables|/Script/Engine.MovementComponent|SetVelocity (Variables|/Game/Blueprint/BP_Projectile.BP_Projectile_C|GetProjectileMovement _returnvalue) (* (Math|Vector|GetForwardVector (Math|Rotator|FindLookatRotation (.location (Transformation|GetWorldTransform (Variables|Default|GetScene))) (Transformation|GetActorLocation (Variables|Default|GetTarget)))) 1e+03)))))

(fn ConstructionScript
  (|CallParentFunction))